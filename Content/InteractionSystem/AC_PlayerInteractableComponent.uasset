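; Actor component that lets its owning Character interact with nearby actors implementing BPI_Interactable.
; Capsule overlaps maintain a list of interactables in range, treating the last entry as the active one.
; Each list change updates a screen-space widget component, created at BeginPlay, placing a prompt at the active interactable or clearing it.
; IA_Interact plays a pickup montage, whose "Interact" notify sends InteractMessage to the active interactable.
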(event Custom|HandleCapsuleOverlapBegin
  (params (OverlappedComponent :type Primitive%20Component%20Object%20Reference) (OtherActor :type Actor%20Object%20Reference) (OtherComp :type Primitive%20Component%20Object%20Reference) (OtherBodyIndex :type Integer) (bFromSweep :type Boolean) (SweepResult :type Hit%20Result%20Structure%20%28by%20ref%29))
  (if (Utilities|DoesObjectImplementInterface OtherActor "/Game/InteractionSystem/BPI_Interactable.BPI_Interactable_C")
    (Utilities|Array|AddUnique (Variables|Default|GetInteractablesInRange) OtherActor)
    (CallFunction|RenderInteractionWidget)))

(event Custom|HandleCapsuleOverlapEnd
  (params (OverlappedComponent :type Primitive%20Component%20Object%20Reference) (OtherActor :type Actor%20Object%20Reference) (OtherComp :type Primitive%20Component%20Object%20Reference) (OtherBodyIndex :type Integer))
  (if (Utilities|DoesObjectImplementInterface OtherActor "/Game/InteractionSystem/BPI_Interactable.BPI_Interactable_C")
    (Utilities|Array|RemoveItem (Variables|Default|GetInteractablesInRange) OtherActor)
    (CallFunction|RenderInteractionWidget)))

(event Input|EnhancedActionEvents|EnhancedInputActionIA_Interact
  (params (ActionValue :type Boolean) (ElapsedSeconds :type Float%20%28double-precision%29) (TriggeredSeconds :type Float%20%28double-precision%29) (InputAction :type Input%20Action%20Object%20Reference :default "/Game/ThirdPerson/Input/Actions/IA_Interact.IA_Interact"))
  (:Started
    (if (Utilities|Array|IsNotEmpty (Variables|Default|GetInteractablesInRange))
      (bind _notifyname (Animation|Montage|PlayMontage (Variables|/Script/Engine.Character|GetMesh (Variables|Default|GetCharacterRef)) "/Game/CustomAnimation/Anim_PickingUpObject_Montage.Anim_PickingUpObject_Montage")
        (:OnNotifyBegin
          (if (== _notifyname "Interact")
            (Class|BPIInteractable|Interact(Message) (CallFunction|GetActiveInteractable) (Components|GetOwner))))))))

(event EventBeginPlay
  (bind _ascharacter (Utilities|Casting|CastToCharacter (Components|GetOwner)))
  (Variables|Default|SetCharacterRef _ascharacter)
  (Collision|BindEventtoOnComponentBeginOverlap (Variables|/Script/Engine.Character|GetCapsuleComponent _ascharacter) (EventDispatchers|CreateEvent :!event Custom|HandleCapsuleOverlapBegin))
  (Collision|BindEventtoOnComponentEndOverlap (Variables|/Script/Engine.Character|GetCapsuleComponent _ascharacter) (EventDispatchers|CreateEvent :!event Custom|HandleCapsuleOverlapEnd))
  (bind _returnvalue (Game|AddComponentbyClass (Components|GetOwner) "/Script/UMG.WidgetComponent" false))
  (Class|WidgetComponent|SetWidgetSpace _returnvalue "Screen")
  (Class|WidgetComponent|SetDrawSize _returnvalue "(X=250.000000,Y=30.000000)")
  (Variables|Default|SetInteractionWidgetComponent _returnvalue))

(fn RenderInteractionWidget
  (bind _interactionwidgetcomponent (Variables|Default|GetInteractionWidgetComponent))
  (if (Utilities|Array|IsNotEmpty (Variables|Default|GetInteractablesInRange))
    (bind _returnvalue (Game|ConstructObjectfromClass "/Game/InteractionSystem/WB_InteractionWidget.WB_InteractionWidget_C"))
    (UserInterface|SetWidget _interactionwidgetcomponent _returnvalue)
    (Transformation|SetWorldLocation _interactionwidgetcomponent (Transformation|GetActorLocation (CallFunction|GetActiveInteractable)) false false)
    (else
      (UserInterface|SetWidget (Variables|Default|GetInteractionWidgetComponent) 0))))

(fn GetActiveInteractable
  (bind _interactablesinrange (Variables|Default|GetInteractablesInRange))
  (return (Utilities|Array|Get(acopy) _interactablesinrange (Utilities|Array|LastIndex _interactablesinrange))))